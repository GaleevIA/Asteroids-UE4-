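; Player-controlled spaceship pawn that strafes along its right vector and fires Plasma_Bolt actors from its own transform.
; Health is a two-hit flag: the first TakeDamage sets IsDamaged and activates a damage particle system, the second calls OnDeath, and HealDamage clears that state.
; OnDeath spawns an emitter, hides the ship, disables collision and sets a delayed RestartGame timer on the game mode.
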(event EventBeginPlay)

(event Collision|EventActorBeginOverlap
  (params (OtherActor :type Actor%20Object%20Reference)))

(event EventTick
  (params (DeltaSeconds :type Float%20%28single-precision%29)))

(event Input|ActionEvents|InputActionShoot
  (params (Key :type Key%20Structure :default "None"))
  (:Pressed
    (Game|SpawnActorfromClass "/Game/Blueprints/Plasma_Bolt.Plasma_Bolt_C" (Transformation|GetActorTransform) "Undefined" 0 0)))

(event Input|AxisEvents|InputAxisMoveRIght
  (params (AxisValue :type Float%20%28single-precision%29))
  (Pawn|Input|AddMovementInput (Transformation|GetActorRightVector) AxisValue false))

(fn ConstructionScript)

(fn TakeDamage
  (if (Variables|Default|GetIsDamaged)
    (CallFunction|OnDeath)
    (else
      (Variables|Default|SetIsDamaged true)
      (Components|Activation|Activate (Variables|Default|GetDamageParticleSystem) false))))

(fn OnDeath
  (Effects|SpawnEmitteratLocation 0 (Transformation|GetActorLocation))
  (Rendering|SetActorHiddenInGame true)
  (Collision|SetActorEnableCollision false)
  (Utilities|Time|SetTimerbyFunctionName (Game|GetGameMode) "RestartGame" 3.0))

(fn HealDamage
  (Variables|Default|SetIsDamaged false)
  (Components|Activation|Deactivate (Variables|Default|GetDamageParticleSystem)))