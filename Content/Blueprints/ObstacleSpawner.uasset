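; ObstacleSpawner is an actor that repeatedly spawns asteroids or health pickups at its own transform.
; On BeginPlay it starts a timer for Spawn with a random delay between its minimum and maximum spawn times.
; Each Spawn call rolls against HealthPickupProbability to choose Health_Pickup or Asteroid, then re-arms the timer with a new random delay, keeping the spawn rhythm irregular.
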(event EventBeginPlay
  (Utilities|Time|SetTimerbyFunctionName 0 "Spawn" (Math|Random|RandomFloatinRange (Variables|Default|GetSpawnTimeMin) (Variables|Default|GetSpawnTimeMax))))

(event Collision|EventActorBeginOverlap
  (params (OtherActor :type Actor%20Object%20Reference)))

(event EventTick
  (params (DeltaSeconds :type Float%20%28single-precision%29)))

(fn ConstructionScript)

(fn Spawn
  (if (>= (Math|Random|RandomFloat) (Variables|Default|GetHealthPickupProbability))
    (Game|SpawnActorfromClass "/Game/Blueprints/Asteroid.Asteroid_C" (Transformation|GetActorTransform) "Undefined" 0 0)
    (else
      (Game|SpawnActorfromClass "/Game/Blueprints/Health_Pickup.Health_Pickup_C" (Transformation|GetActorTransform) "Undefined" 0 0)))
  (Utilities|Time|SetTimerbyFunctionName 0 "Spawn" (Math|Random|RandomFloatinRange (Variables|Default|GetSpawnTimeMin) (Variables|Default|GetSpawnTimeMax))))