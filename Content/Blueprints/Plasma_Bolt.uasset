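; Plasma bolt projectile actor that destroys asteroids on contact.
; On overlap with an Asteroid, it spawns the P_Explosion particle effect at the asteroid's location, then destroys both the asteroid and itself.
; Overlaps with other actors are ignored, and its graphs contain no movement, BeginPlay or Tick logic.
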(event EventBeginPlay
  (|CallParentFunction) ; This node is disabled and will not be called.\nDrag off pins to build functionality.
)

(event Collision|EventActorBeginOverlap
  (params (OtherActor :type Actor%20Object%20Reference))
  (bind _asasteroid (Utilities|Casting|CastToAsteroid OtherActor))
  (Effects|SpawnEmitteratLocation "/Game/StarterContent/Particles/P_Explosion.P_Explosion" (Transformation|GetActorLocation _asasteroid))
  (Actor|DestroyActor _asasteroid)
  (Actor|DestroyActor))

(event EventTick
  (params (DeltaSeconds :type Float%20%28single-precision%29))
  (|CallParentFunction DeltaSeconds) ; This node is disabled and will not be called.\nDrag off pins to build functionality.
)

(fn ConstructionScript
  (|CallParentFunction))